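; BP_Pawn is a Blueprint that hides its Cylinder when the cursor trace matches it, and whitens its Cube.
; Each tick, a complex Visibility trace under player 0's cursor stores the hit actor in PawnActor and compares it to Cylinder, with no path to re-show it.
; The construction script creates a dynamic MAT_White instance on CubeMaterial, but assigns MAT_White itself to Cube.
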(event EventTick
  (params (DeltaSeconds :type Float%20%28single-precision%29))
  (bind _returnvalue (Game|GetPlayerController 0))
  (bind (_hitresult _returnvalue_2) (Game|Player|GetHitResultUnderCursorbyChannel _returnvalue "TraceTypeQuery1" true))
  (if _returnvalue_2
    (bind _output_get (Variables|Default|SetPawnActor (.HitActor (Collision|BreakHitResult _hitresult))))
    (if (== (Variables|Default|GetCylinder) _output_get)
      (Rendering|SetVisibility (Variables|Default|GetCylinder) false false))))

(fn ConstructionScript
  (Rendering|Material|CreateDynamicMaterialInstance (Variables|Default|GetCubeMaterial) 0 "/Game/Week7/MAT_White.MAT_White" :!class /Script/Engine.PrimitiveComponent)
  (Rendering|Material|SetMaterial (Variables|Default|GetCube) 0 "/Game/Week7/MAT_White.MAT_White"))